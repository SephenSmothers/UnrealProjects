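; BP_Agent is an AI-controlled armed agent with a weapon, a health component and a color applied to its mesh materials.
; On begin play it binds weapon and health delegates and loads ammo; update functions write health and ammo to the AI controller's Blackboard.
; EnemyAttack and EnemyReload drive the weapon, and EndAttack sends an AI finish message.
; Tick also calls Attack every frame, independently of EnemyAttack.
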(event Custom|EndAttack
  (Class|AIBlueprintHelperLibrary|SendAIMessage self (Variables|Default|GetAIFinishMessage) 0 true))

(event EventBeginPlay
  (bind _weapon (Variables|Default|GetWeapon))
  (|CallParentFunction)
  (Rendering|Material|SetVectorParameterValueonMaterials (Variables|Character|GetMesh) "None" (Math|Conversions|ToVector(LinearColor) (Variables|Default|GetColor)))
  (EventDispatchers|BindEventtoOnActionStopped (Variables|Default|GetWeapon) (EventDispatchers|CreateEvent :!event Custom|EndAttack))
  (EventDispatchers|BindEventtoOnHurt (Variables|Default|GetBP_HealthComponent) (EventDispatchers|CreateEvent :!event UpdateHealth))
  (CallFunction|UpdateHealth 1.0)
  (EventDispatchers|BindEventtoOnAmmoChanged _weapon (EventDispatchers|CreateEvent :!event UpdateAmmo))
  (Default|ReloadAmmo _weapon))

(event Collision|EventActorBeginOverlap
  (params (OtherActor :type Actor%20Object%20Reference)))

(event EventTick
  (params (DeltaSeconds :type Float%20%28single-precision%29))
  (|CallParentFunction DeltaSeconds)
  (Default|Attack (Variables|Default|GetWeapon)))

(event EventEnemyAttack
  (Default|Attack (Variables|Default|GetWeapon)))

(event EventEnemyReload
  (Default|RequestReload (Variables|Default|GetWeapon)))

(fn ConstructionScript
  (|CallParentFunction))

(fn UpdateHealth
  (params (Percentage :type Float%20%28single-precision%29))
  (AI|Components|Blackboard|SetValueasFloat (AI|GetBlackboard (AI|GetAIController self)) (Variables|Default|GetHealthName) Percentage))

(fn UpdateAmmo
  (params (Current :type Float%20%28single-precision%29) (Max :type Float%20%28single-precision%29))
  (AI|Components|Blackboard|SetValueasFloat (AI|GetBlackboard (AI|GetAIController self)) (Variables|Default|GetAmmoName) Current))