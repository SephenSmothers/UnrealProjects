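; Rifle actor held by a parent Pawn that fires projectiles and tracks ammo, destroying itself on BeginPlay if no Pawn parent exists.
; Attack spawns a projectile at the muzzle socket along the Pawn's aim, gated by ammo, owner-alive state and a busy flag.
; A timer follows each shot, while reload refills ammo instantly and sets the busy flag.
; Event dispatchers broadcast firing, reload start, action stop and ammo changes.
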(event Custom|ActionStopped
  (Variables|Default|SetActionHappening false)
  (Default|CallOnActionStopped))

(event Custom|OwnerDied
  ;[1 0 0.06124] Comment
  (Variables|Default|SetOwnerAlive false))

(event Custom|ReloadAmmo
  (bind _maxammo (Variables|Default|GetMaxAmmo))
  (bind _output_get (Variables|Default|SetCurrentAmmo _maxammo))
  (Default|CallOnAmmoChanged _output_get _maxammo))

(event Custom|UseAmmo
  (bind _output_get (Variables|Default|SetCurrentAmmo (Math|Float|Max(Float) (- (Variables|Default|GetCurrentAmmo) 1.0) 0.0)))
  (Default|CallOnAmmoChanged _output_get (Variables|Default|GetMaxAmmo)))

(event Custom|RequestReload
  (if (not (Variables|Default|GetActionHappening))
    (Variables|Default|SetActionHappening true)
    (CallFunction|ReloadAmmo)
    (Default|CallOnReloadStart)))

(event EventBeginPlay
  (bind _aspawn (Utilities|Casting|CastToPawn (Actor|GetParentActor))
    (:then
      (Variables|Default|SetParentPawn _aspawn)
      (CallFunction|ReloadAmmo))
    (:CastFailed
      (Development|PrintString "The Rifel Needs to be held by a Pawn")
      (Actor|DestroyActor))))

(fn ConstructionScript)

(fn Attack
  (bind _parentpawn (Variables|Default|GetParentPawn))
  (if (CallFunction|CanShoot)
    (Game|SpawnActorfromClass (Variables|Default|GetProjectileClass) (Math|Transform|MakeTransform (Transformation|GetSocketLocation (Variables|Default|GetSkeletalMesh) "MuzzleFlashSocket") (Pawn|GetBaseAimRotation _parentpawn) "1,1,1") "Undefined" (Pawn|GetController _parentpawn) _parentpawn)
    (Variables|Default|SetActionHappening true)
    (Utilities|Time|SetTimerbyEvent (EventDispatchers|CreateEvent :!event Custom|ActionStopped) (Variables|Default|GetTime))
    (Default|CallOnRifleFire)
    (CallFunction|UseAmmo)))

(fn CanShoot
  (return (Math|Boolean|ANDBoolean (not (Variables|Default|GetActionHappening)) (Variables|Default|GetOwnerAlive) (> (Variables|Default|GetCurrentAmmo) 0.0))))