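; Game mode that tracks win and lose conditions for a match between the player and enemy characters.
; On BeginPlay it finds all base characters, stores the player, binds to its end-game event, counts enemies via their destroy events and creates the results widget.
; Player loss unbinds destroy events, stops AI logic and shows results with UI-only input.
; Destroying the last enemy prints a win and shows the same widget.
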(event Custom|RemovePlayer
  (bind _currentcontroller (Variables|Default|GetCurrentController))
  (Development|PrintString "You Lose")
  (bind _outactors (Actor|GetAllActorsOfClass "/Game/BluePrints/Actors/BP_BaseCharacter.BP_BaseCharacter_C"))
  (for _array_element _outactors
    (Game|UnbindEventfromOnDestroyed _array_element (EventDispatchers|CreateEvent :!event RemoveEnemy))
    (Utilities|IsValid (AI|GetAIController _array_element)
      (:Is%20Valid
        (AI|Logic|StopLogic (Variables|/Script/AIModule.AIController|GetBrainComponent (AI|GetAIController _array_element)) "Player Is Dead"))))
  (UserInterface|Viewport|AddtoViewport (Variables|Default|GetResultWidget) 0)
  (Variables|/Script/Engine.PlayerController|SetbShowMouseCursor _currentcontroller true)
  (Input|SetInputModeUIOnly _currentcontroller (Variables|Default|GetResultWidget) "LockAlways"))

(event EventBeginPlay
  (bind _outactors (Actor|GetAllActorsOfClass "/Game/BluePrints/Actors/BP_BaseCharacter.BP_BaseCharacter_C"))
  (for _array_element _outactors
    (bind _asbp_player (Utilities|Casting|CastToBP_Player _array_element)
      (:then
        (Variables|Default|SetCurrentPlayer _asbp_player)
        (EventDispatchers|BindEventtoOnEndGame _asbp_player (EventDispatchers|CreateEvent :!event Custom|RemovePlayer)))
      (:CastFailed
        (CallFunction|AddEnemy _array_element))))
  (bind _returnvalue (Actor|GetActorOfClass (Variables|Default|GetPlayerControllerClass)))
  (bind _output_get (Variables|Default|SetCurrentController _returnvalue))
  (bind _returnvalue_2 (UserInterface|CreateWidget (Variables|Default|GetResultsWidgetClass) _output_get))
  (Variables|Default|SetResultWidget _returnvalue_2))

(fn ConstructionScript)

(fn AddEnemy
  (params (Actor :type Actor%20Object%20Reference))
  (Math|Integer|IncrementInt (Variables|Default|GetNumEnemies)
    (:%20%20
      (Game|BindEventtoOnDestroyed Actor (EventDispatchers|CreateEvent :!event RemoveEnemy)))))

(fn RemoveEnemy
  (params (DestroyedActor :type Actor%20Object%20Reference))
  (bind _result (Math|Integer|DecrementInt (Variables|Default|GetNumEnemies))
    (:%20%20
      (if (not (> _result 0))
        (Development|PrintString "You Win")
        (UserInterface|Viewport|AddtoViewport (Variables|Default|GetResultWidget) 0)))))