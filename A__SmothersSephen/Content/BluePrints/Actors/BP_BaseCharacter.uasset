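; BP_BaseCharacter is a base character that carries a rifle and responds to hurt and death events.
; On begin play it spawns the weapon class through a child actor component, caches the rifle and animation Blueprint, and destroys itself if either cast fails.
; It binds handlers to rifle fire and to health component hurt and death dispatchers.
; Death handling disables collision and notifies the weapon that its owner died.
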(event Custom|HandleDeath
  (params (Ratio :type Float%20%28single-precision%29))
  ;[1 0.239 0.2291] Comment
  (Collision|SetActorEnableCollision false)
  (Default|OwnerDied (Variables|Default|GetWeapon)))

(event EventBeginPlay
  (bind _childactorcomponent (Variables|Default|GetChildActorComponent))
  (bind _bp_healthcomponent (Variables|Default|GetBP_HealthComponent))
  (ChildActorComponent|SetChildActorClass _childactorcomponent (Variables|Default|GetWeaponClass))
  (bind _asbp_rifle (Utilities|Casting|CastToBP_Rifle (Variables|/Script/Engine.ChildActorComponent|GetChildActor _childactorcomponent))
    (:then
      (Variables|Default|SetWeapon _asbp_rifle)
      (bind _asabp_character_animation (Utilities|Casting|CastToABP_CharacterAnimation (Components|SkeletalMesh|GetAnimInstance (Variables|Character|GetMesh)))
        (:then
          (Variables|Default|SetAnimInstanceBP _asabp_character_animation)
          (EventDispatchers|BindEventtoOnRifleFire (Variables|Default|GetWeapon) (EventDispatchers|CreateEvent (Variables|Default|GetAnimInstanceBP) :!event FireAnimation))
          ;[1 0.239 0.2291] Comment
          (EventDispatchers|BindEventtoOnHurt _bp_healthcomponent (EventDispatchers|CreateEvent (Variables|Default|GetAnimInstanceBP) :!event HurtAnimation))
          (EventDispatchers|BindEventtoOnDead _bp_healthcomponent (EventDispatchers|CreateEvent (Variables|Default|GetAnimInstanceBP) :!event DeadAnimation))
          (EventDispatchers|BindEventtoOnDead _bp_healthcomponent (EventDispatchers|CreateEvent :!event Custom|HandleDeath)))
        (:CastFailed
          (Development|PrintString "Worng Anim Clas Set")
          (Actor|DestroyActor))))
    (:CastFailed
      (Development|PrintString "We need a Rifle Class For the Base Character")
      (Actor|DestroyActor))))

(fn ConstructionScript)