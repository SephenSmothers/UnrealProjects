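; BP_BasePickup is a base pickup actor with overridable hooks for what happens when something overlaps it.
; The construction script binds the box collision's begin-overlap event, and HandleOverlap calls an empty HandlePickup, then HandlePostPickup, which destroys the actor.
; CanPickup returns false but is not wired into that flow, so any overlap that reaches HandleOverlap consumes the pickup unconditionally.
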(event EventBeginPlay)

(event Collision|EventActorBeginOverlap
  (params (OtherActor :type Actor%20Object%20Reference)))

(event EventTick
  (params (DeltaSeconds :type Float%20%28single-precision%29)))

(fn ConstructionScript
  (Collision|BindEventtoOnComponentBeginOverlap (Variables|Default|GetBoxCollision) (EventDispatchers|CreateEvent :!event HandleOverlap)))

(fn HandleOverlap
  (params (OverlappedComponent :type Primitive%20Component%20Object%20Reference) (OtherActor :type Actor%20Object%20Reference) (OtherComp :type Primitive%20Component%20Object%20Reference) (OtherBodyIndex :type Integer) (bFromSweep :type Boolean) (SweepResult :type Hit%20Result%20Structure%20%28by%20ref%29))
  (CallFunction|HandlePickup OtherActor SweepResult)
  (CallFunction|HandlePostPickup)
  (return))

(fn HandlePickup
  (params (OtherActor :type Actor%20Object%20Reference) (SweepResult :type Hit%20Result%20Structure)))

(fn HandlePostPickup
  (Actor|DestroyActor))

(fn CanPickup
  (params (OtherActor :type Actor%20Object%20Reference))
  (return false))