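; BP_Projectile is a projectile actor that destroys itself when its overlap handler fires.
; On BeginPlay it starts a one-shot timer of DestroyTimer length, apparently to limit its lifetime.
; The construction script binds an event to the sphere collision's begin overlap and scales that sphere by the Size variable.
; The graphs contain no movement or damage logic.
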(event Custom|HandleOverlap
  (params (OverlappedComponent :type Primitive%20Component%20Object%20Reference) (OtherActor :type Actor%20Object%20Reference) (OtherComp :type Primitive%20Component%20Object%20Reference) (OtherBodyIndex :type Integer) (bFromSweep :type Boolean) (SweepResult :type Hit%20Result%20Structure%20%28by%20ref%29))
  (Actor|DestroyActor))

(event EventBeginPlay
  (Utilities|Time|SetTimerbyEvent (EventDispatchers|CreateEvent :!event K2DestroyActor) (Variables|Default|GetDestroyTimer)))

(fn ConstructionScript
  (Collision|BindEventtoOnComponentBeginOverlap (Variables|Default|GetSphereCollision) (EventDispatchers|CreateEvent :!event Custom|HandleOverlap))
  (Transformation|SetWorldScale3D (Variables|Default|GetSphereCollision) (Variables|Default|GetSize)))