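; Game instance Blueprint that handles level flow: loading the first level, main menu or current level, and quitting the game.
; Its load events pass stored indices to LoadLevel, which validates them against the GameLevels array and records the current index.
; OpenLevelByName receives "None", as the GameLevels lookup is left unconnected.
; Invalid indices only print a debug string.
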(event Custom|LoadFirstLevel
  (CallFunction|LoadLevel (Variables|Default|GetFirstLevelIndex)))

(event Custom|QuitGame
  (Game|QuitGame 0 "Quit" false))

(event Custom|LoadMainMenu
  (CallFunction|LoadLevel (Variables|Default|GetMainMenuIndex)))

(event Custom|LoadCurrentLevel
  (CallFunction|LoadLevel (Variables|Default|GetCurrentLevelIndex)))

(fn LoadLevel
  (params (LevelIndex :type Integer))
  (if (Utilities|Array|IsValidIndex (Variables|Default|GetGameLevels) LevelIndex)
    (bind _output_get (Variables|Default|SetCurrentLevelIndex LevelIndex))
    (Game|OpenLevel(byName) "None")
    (else
      (Development|PrintString "stuff happened"))))